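; Sword combat character Blueprint shared by the player and "Enemy"-tagged AI, branching setup on BeginPlay by tag and controller.
; Enemies equip twin blades and show a health bar that yaws toward the player; the player gets screen UI and tracks nearby actors through a sense trigger.
; The player also toggles an inventory widget and drinks skill-slot potions to heal.
; On death, the character is unpossessed.
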(event `self.ReceiveTick`
  (params (DeltaSeconds :type "Float (single-precision)"))
  (if (`self.bIsDeath`)
    (`/Engine/EditorBlueprintResources/StandardMacros.DoOnce` false
      (:`Completed`
        (`self.UnPossesCharacter`)))
    (elif (not (`Controller.IsPlayerController` (`self.GetController`)))
      (`self.RotateHealthBarThroughPlayer`)
      (`self.DisplayCurrentHealth`))))

(event `self.ReceiveBeginPlay`
  (`self.ConstructAIEnemy`)
  (`self.ConstructPlayer`))

(event `InputAction|Inventory`
  (params (Key :type "Key Structure"))
  (:`Pressed`
    (`self.InventoryToggle`)))

(event `self.PlayerSenseTrigger.OnComponentBeginOverlap`
  (params (OverlappedComponent :type "PrimitiveComponent Object Reference") (OtherActor :type "Actor Object Reference") (OtherComp :type "PrimitiveComponent Object Reference") (OtherBodyIndex :type Integer) (bFromSweep :type Boolean) (SweepResult :type "HitResult Structure (by ref)"))
  (`self.AddActorToCloseAttackerList` OtherActor))

(event `self.PlayerSenseTrigger.OnComponentEndOverlap`
  (params (OverlappedComponent :type "PrimitiveComponent Object Reference") (OtherActor :type "Actor Object Reference") (OtherComp :type "PrimitiveComponent Object Reference") (OtherBodyIndex :type Integer))
  (`self.RemoveActorFromCloseAttackerList` OtherActor))

(event `OnItemAddToSkillCaster`
  (params (Item :type "InventoryItem Structure"))
  (set `self.PotionQuantitiy` Item_Quantity)
  (`/Game/Character/UI/Player/SkillCastingUI.OnSkillEquiped` (`/Game/Character/UI/Player/CharacterUI.SkillCastingUI` (`self.CharacterUI`)) (make `InventoryItem` Item_ItemClass Item_ItemType Item_Name Item_Quantity Item_Slot Item_Image)))

(event `Key|One`
  (params (Key :type "Key Structure"))
  (:`Pressed`
    (if (and (`self.IsHavePotion`) (> (`self.PotionQuantitiy`) 0))
      (set `self.CurrentHealth` (+ (`self.CurrentHealth`) 30.0))
      (`/Engine/EditorBlueprintResources/StandardMacros.DecrementInt` (`self.PotionQuantitiy`)))))

(fn `ConstructAIEnemy`
  (if (`self.ActorHasTag` "Enemy")
    (`Inventory.SetPrimaryWeapon` (`self.CharacterInventory`) null)
    (`self.EquipWeapon` "/Game/Weapons/TwinBlades/BP_TwinBlades.BP_TwinBlades_C")
    (`self.SetAnimationInstance` "/Game/Character/Animations/TwinBladesSwordAnimations/ABP_TwinBlades.ABP_TwinBlades_C")
    (`CombatState.DrawPrimaryWeapon` (`self.CombatState`))
    (`ActorComponent.K2_DestroyComponent` (`self.PlayerSenseTrigger`))))

(fn `ConstructPlayer`
  (bind _returnvalue (`GameplayStatics.GetPlayerController` 0))
  (bind _playersensetrigger (`self.PlayerSenseTrigger`))
  (if (`Controller.IsPlayerController` (`self.GetController`))
    (`/Engine/EditorBlueprintResources/StandardMacros.IsValid` _playersensetrigger
      (:`Is Valid`
        (set `PrimitiveComponent.bGenerateOverlapEvents` true _playersensetrigger)
        (`ActorComponent.K2_DestroyComponent` (`self.HealthBar`))
        (bind _returnvalue_2 (`|CreateWidget` "/Game/Character/UI/Player/PlayerHealthBar.PlayerHealthBar_C" _returnvalue))
        (`UserWidget.AddToViewport` _returnvalue_2 1)
        (bind _returnvalue_3 (`|CreateWidget` "/Game/Character/UI/Player/CharacterUI.CharacterUI_C" _returnvalue))
        (bind _output_get (set `self.CharacterUI` _returnvalue_3))
        (`UserWidget.AddToViewport` _output_get 0)))))

(fn `DisplayCurrentHealth`
  (bind _ashealth_bar (cast `/Game/Character/UI/HealthBar` (`WidgetComponent.GetUserWidgetObject` (`self.HealthBar`))))
  (`ProgressBar.SetPercent` (`/Game/Character/UI/HealthBar.HealthBar` _ashealth_bar) (/ (`self.CurrentHealth`) (`self.MaxHealth`))))

(fn `InventoryUIToggle`)

(fn `RotateHealthBarThroughPlayer`
  (bind _returnvalue (`GameplayStatics.GetPlayerCharacter` 0))
  (`/Engine/EditorBlueprintResources/StandardMacros.IsValid` _returnvalue
    (:`Is Valid`
      (`SceneComponent.K2_SetWorldRotation` (`self.HealthBar`) (`KismetMathLibrary.MakeRotator` 0.0 0.0 (.yaw (`KismetMathLibrary.FindLookAtRotation` (`SceneComponent.K2_GetComponentLocation` (`self.HealthBar`)) (`self.K2_GetActorLocation` _returnvalue)))) false false))))

(fn `UnPossesCharacter`
  (bind _returnvalue (`self.GetController`))
  (bind _output_get (set `self.IsPlayerController` (`Controller.IsPlayerController` _returnvalue)))
  (`Controller.UnPossess` _returnvalue)
  (if (not _output_get)
    (`ActorComponent.K2_DestroyComponent` (`self.HealthBar`))))

(fn `UserConstructionScript`)